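; Ground_BP is a construction-time actor that lays out a straight strip of ground pieces from one instanced static mesh.
; The construction script sets the mesh from the Mesh array, either randomly among the first three entries when RandomMeshMaterial is on or by MeshId.
; It then loops over GroundCount to add instances at even spacing along local X, with one mesh shared by the whole strip.
; The event graph holds no active logic.
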(event EventBeginPlay)

(event Collision|EventActorBeginOverlap
  (params (OtherActor :type Actor%20Object%20Reference)))

(event EventTick
  (params (DeltaSeconds :type Float%20%28single-precision%29)))

(fn ConstructionScript
  (bind _mesh (Variables|Default|GetMesh))
  (bind _instancedstaticmesh (Variables|Default|GetInstancedStaticMesh))
  (Utilities|FlowControl|Sequence
    (:then_0
      (if (Variables|Default|GetRandom_mesh_material)
        (Components|StaticMesh|SetStaticMesh _instancedstaticmesh (Utilities|Array|Get(acopy) _mesh (Math|Random|RandomIntegerinRange 0 2)))
        (else
          (Components|StaticMesh|SetStaticMesh _instancedstaticmesh (Utilities|Array|Get(acopy) _mesh (Variables|Default|GetMesh_id))))))
    (:then_1
      (for _index (range 0 (Variables|Default|Getground_count))
        (Components|InstancedStaticMesh|AddInstance (Variables|Default|GetInstancedStaticMesh) (Math|Transform|MakeTransform (Math|Vector|MakeVector (* _index 1e+02) 0.0 0.0)) false)))))