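; Arm door Blueprint for the jail that reacts to a key and to a doctor actor.
; Tick watches for KeyChild becoming invalid, then once snaps the door to zero rotation with the DoorClosed sound and swings it to a quarter-turn yaw after a long delay.
; Separately, an actor tagged Doctor entering the Box trigger is destroyed, and a knocking sound plays for a few seconds.
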(event OnComponentBeginOverlap(Box)
  (params (OverlappedComponent :type Primitive%20Component%20Object%20Reference) (OtherActor :type Actor%20Object%20Reference) (OtherComp :type Primitive%20Component%20Object%20Reference) (OtherBodyIndex :type Integer) (bFromSweep :type Boolean) (SweepResult :type Hit%20Result%20Structure%20%28by%20ref%29))
  (bind _knockingdoor (Variables|Default|GetknockingDoor))
  (if (Actor|ActorHasTag OtherActor "Doctor")
    (Actor|DestroyActor OtherActor)
    (Audio|Components|Audio|Play _knockingdoor 0.0)
    (Utilities|FlowControl|Delay 6.0)
    (Audio|Components|Audio|Stop _knockingdoor)))

(event EventTick
  (params (DeltaSeconds :type Float%20%28single-precision%29))
  (bind _door (Variables|Default|GetDoor))
  (if (not (Utilities|IsValid (Variables|Default|GetKeyChild)))
    (Utilities|FlowControl|DoOnce false
      (:Completed
        (Transformation|SetRelativeRotation _door (Math|Rotator|MakeRotator 0.0 0.0 0.0) false false)
        (Audio|Components|Audio|Play (Variables|Default|GetDoorClosed) 0.0)
        (Utilities|FlowControl|Delay 21.0)
        (Transformation|SetRelativeRotation _door (Math|Rotator|MakeRotator 0.0 0.0 -9e+01) false false)))))

(fn ConstructionScript)