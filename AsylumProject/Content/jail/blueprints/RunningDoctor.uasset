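; RunningDoctor is a one-shot scare or scripted-event actor in the jail level that shows a doctor running when the player enters its trigger.
; On overlap with a Player-tagged actor, it reveals the skeletal mesh, loops the running animation, starts InterpToMovement and plays audio.
; The actor destroys itself after a delay equal to the movement duration.
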(event OnComponentBeginOverlap(Trigger)
  (params (OverlappedComponent :type Primitive%20Component%20Object%20Reference) (OtherActor :type Actor%20Object%20Reference) (OtherComp :type Primitive%20Component%20Object%20Reference) (OtherBodyIndex :type Integer) (bFromSweep :type Boolean) (SweepResult :type Hit%20Result%20Structure%20%28by%20ref%29))
  (bind _skeletalmesh (Variables|Default|GetSkeletalMesh))
  (if (Actor|ActorHasTag OtherActor "Player")
    (Rendering|SetVisibility _skeletalmesh true false)
    (Components|Animation|PlayAnimation _skeletalmesh "/Game/Animations/Doctor/Running.Running" true)
    (Components|Activation|Activate (Variables|Default|GetInterpToMovement) false)
    (Audio|Components|Audio|Play (Variables|Default|GetAudio) 0.0)
    (Utilities|FlowControl|Delay (Variables|/Script/Engine.InterpToMovementComponent|GetDuration (Variables|Default|GetInterpToMovement)))
    (Actor|DestroyActor)))

(fn ConstructionScript)