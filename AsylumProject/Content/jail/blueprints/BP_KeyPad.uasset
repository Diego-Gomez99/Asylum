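; BP_KeyPad is a keypad actor that takes PIN input from the player to unlock a linked BP_Door.
; Entering its view blends the camera to the keypad and switches to UI-only input with a visible cursor.
; On BeginPlay it registers itself with its KeyPadWidget, then forwards received pin values to the door's AddToPin.
; On success it tells the widget to exit, applies a green light material and sets the player's HasKey.
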(event EventBeginPlay
  (bind _asbp_first_person_character (Utilities|Casting|CastToBP_FirstPersonCharacter (Game|GetPlayerCharacter 0)))
  (Variables|Default|SetPlayerRef _asbp_first_person_character)
  (Variables|/Game/Widgets/KeyPadWidget.KeyPadWidget_C|SetBP_KeyPad (.AsKey%20Pad%20Widget (Utilities|Casting|CastToKeyPadWidget (UserInterface|GetUserWidgetObject (Variables|Default|GetWidget)))) self))

(event EventGetPinValue
  (params (Pin%20Value :type String))
  (bind _ispincorrect_ (Default|AddtoPin (.AsBP%20Door (Utilities|Casting|CastToBP_Door (Variables|Default|GetDoorActor))) Pin%20Value))
  (if _ispincorrect_
    (Default|ExitKeypadView (.AsKey%20Pad%20Widget (Utilities|Casting|CastToKeyPadWidget (UserInterface|GetUserWidgetObject (Variables|Default|GetWidget)))))
    (Rendering|Material|SetMaterial (Variables|Default|GetStaticMesh) 0 "/Game/jail/materials/Light_door_Green_mat.Light_door_Green_mat")
    (Variables|/Script/AsylumProject.AsylumProjectCharacter|SetHasKey (Variables|Default|GetPlayerRef) true)))

(fn ConstructionScript)

(fn EnterKeypadView
  (bind _returnvalue (Game|GetPlayerController 0))
  (Game|Player|SetViewTargetwithBlend _returnvalue self (Variables|Default|GetBlendTime) "VTBlend_Linear" 0.0 false)
  (Input|SetInputModeUIOnly _returnvalue 0 "DoNotLock" false)
  (Variables|/Script/Engine.PlayerController|SetbShowMouseCursor _returnvalue true))