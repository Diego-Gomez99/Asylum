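; A wall entry light Blueprint for the jail, with a mesh and point light that can flicker or shift color.
; The construction script sets the mesh material from an array and hides the point light when the Light flag is true.
; FlickeringLight blinks the light off and on with a sound after a random delay, calling itself while CanLighFlick holds.
; TurnRedLight and TurnNormalLight drive the light color through timelines.
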(event Custom|FlickeringLight
  (bind _pointlight (Variables|Default|GetPointLight))
  (Utilities|FlowControl|Delay (Math|Conversions|ToFloat(Integer) (Math|Random|RandomInteger 10)))
  (Rendering|SetVisibility _pointlight false false)
  (Utilities|FlowControl|Delay 0.2)
  (Rendering|SetVisibility _pointlight true false)
  (Audio|PlaySoundatLocation "/Game/Sounds/FlickeringLightCue.FlickeringLightCue" (Transformation|GetWorldLocation _pointlight) "0, 0, 0" 1.0 1.0 0.0 0 0 0 0)
  (Utilities|FlowControl|Delay 0.1)
  (if (Variables|Default|GetCanLighFlick)
    (CallFunction|FlickeringLight)))

(event Custom|TurnRedLight
  (bind _colortrack (Timeline|TurntoRedColor Play)
    (:Update
      (Rendering|Components|Light|SetLightColor (Variables|Default|GetPointLight) _colortrack true))))

(event Custom|TurnNormalLight
  (bind _colortrack (Timeline|TurnNormalColor Play)
    (:Update
      (Rendering|Components|Light|SetLightColor (Variables|Default|GetPointLight) _colortrack true))))

(fn ConstructionScript
  (Utilities|FlowControl|Sequence
    (:then_0
      (Rendering|Material|SetMaterial))
    (:then_1
      (|Visibility))))