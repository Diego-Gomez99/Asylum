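; BP_Door is a lockable door with a hand-icon widget whose visibility can be toggled.
; ChangeDoorIcon takes a HasKey flag: with a key it shows the open icon, plays the unlock sound and alternately plays or reverses a timeline that lerps the mesh yaw between closed and open angles.
; Without a key it plays the locked sound and shows a padlock icon for one second.
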(event Custom|ChangeDoorIcon
  (params (HasKey? :type Boolean))
  (bind _returnvalue (Transformation|GetActorLocation))
  ;[1 1 1] Door Interaction
  (bind _asdoor_interact_widget (Utilities|Casting|CastToDoorInteractWidget (UserInterface|GetWidget (Variables|Default|GetHandWidget))))
  (if HasKey?
    (Default|GetIcon _asdoor_interact_widget "/Game/Widgets/OpenDoor.OpenDoor")
    (Audio|PlaySoundatLocation "/Game/Sounds/DoorUnlockedCue.DoorUnlockedCue" _returnvalue "0, 0, 0" 1.0 1.0 0.0 0 0 0 0)
    (Utilities|FlowControl|FlipFlop
      (:A
        (bind _door_track (Timeline|Open/Close%20Door Play)
          (:Update
            (Transformation|SetRelativeRotation (Variables|Default|GetDoorMesh) (Math|Rotator|MakeRotator 0.0 0.0 (Math|Float|Lerp (Variables|Default|GetClosedAngle) (Variables|Default|GetOpenAngle) _door_track)) false false))))
      (:B
        (Timeline|Open/Close%20Door Reverse)))
    (else
      (Default|GetIcon _asdoor_interact_widget "/Game/Widgets/PadLockIcon.PadLockIcon")
      (Audio|PlaySoundatLocation "/Game/Sounds/DoorLockedCue.DoorLockedCue" _returnvalue "0, 0, 0" 1.0 1.0 0.0 0 0 0 0)
      (Utilities|FlowControl|Delay 1.0)
      (Default|GetIcon _asdoor_interact_widget "/Game/Widgets/OpenDoor.OpenDoor"))))

(fn ConstructionScript)

(fn WidgetDoorVisibility
  (params (IsVisibility :type Boolean))
  (Rendering|SetVisibility (Variables|Default|GetHandWidget) IsVisibility false))